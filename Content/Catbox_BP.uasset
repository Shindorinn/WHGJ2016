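; Interactable catbox whose door opens once when the interaction runs.
; ExecuteInteraction sets a one-time flag, plays the door's skeletal mesh animation and returns true, or returns false if already opened.
; It also fires HideCollisionEvent, which disables the door's separate collision mesh after a short delay.
; RetrieveCatThoughText returns an empty string, so the box supplies no cat thought text.
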(event Custom|HideCollisionEvent
  (Utilities|FlowControl|Delay 0.4)
  (Collision|SetCollisionEnabled (Variables|Default|GetCatDoorCollStaticMesh) "NoCollision"))

(event EventBeginPlay)

(event EventActorBeginOverlap
  (params (OtherActor :type Actor%20Object%20Reference)))

(event EventTick
  (params (DeltaSeconds :type Float%20%28single-precision%29)))

(fn ConstructionScript)

(fn ExecuteInteraction
  (if (Variables|Default|GetHasOpenedDoor)
    (return false)
    (else
      (Variables|Default|SetHasOpenedDoor true)
      (Components|Animation|PlayAnimation (Variables|Default|GetCatboxDoorSkeletalMesh) "/Game/CustomContent/CatBox/CatboxDoor_Anim.CatboxDoor_Anim" false)
      (CallFunction|HideCollisionEvent)
      (return true))))

(fn RetrieveCatThoughText
  (return ""))